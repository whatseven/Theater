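; FPS projectile actor that awards the shooter a point when it hits a target.
; On a collision hit, it checks whether the other actor's object name is exactly "Target", then casts its stored Shooter to ThirdPersonCharacter and increments that character's Score.
; The projectile destroys itself only after a successful score; other hits or a failed cast leave it alive.
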(event `self.collision.OnComponentHit`
  (params (HitComponent :type "PrimitiveComponent Object Reference") (OtherActor :type "Actor Object Reference") (OtherComp :type "PrimitiveComponent Object Reference") (NormalImpulse :type "Vector Structure") (Hit :type "HitResult Structure (by ref)"))
  (if (`KismetStringLibrary.EqualEqual_StrStr` "Target" (`KismetSystemLibrary.GetObjectName` OtherActor))
    (bind _asthird_person_character (cast `/Game/ThirdPersonCPP/Blueprints/ThirdPersonCharacter` (`self.Shooter`)))
    (set `/Game/ThirdPersonCPP/Blueprints/ThirdPersonCharacter.score` (+ (`/Game/ThirdPersonCPP/Blueprints/ThirdPersonCharacter.score` _asthird_person_character) 1) _asthird_person_character)
    (`self.K2_DestroyActor`)))

(event `self.ReceiveBeginPlay`)

(event `self.ReceiveActorBeginOverlap`
  (params (OtherActor :type "Actor Object Reference")))

(event `self.ReceiveTick`
  (params (DeltaSeconds :type "Float (single-precision)")))

(fn `UserConstructionScript`)